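; A mode-selection pawn that lets the player operate widgets with either VR controllers or a mouse.
; Every tick it moves the left and right widget interaction components to each motion controller's aim position and rotation.
; The left and right trigger inputs act as left mouse clicks on their pointers, while the mouse button drives a separate interaction component, pressing only over interactable widgets.
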(event `self.ReceiveTick`
  (params (DeltaSeconds :type "Float (single-precision)"))
  (bind _motioncontrollerright (`self.MotionControllerRight`))
  (bind _motioncontrollerleft (`self.MotionControllerLeft`))
  ;[1 1 1] Update VR's Pointer
  (`|ExecutionSequence`
    (:`then_0`
      (if (`KismetSystemLibrary.IsValid` _motioncontrollerleft)
        (bind _motioncontrollerdata (`HeadMountedDisplayFunctionLibrary.GetMotionControllerData` _motioncontrollerleft "Left"))
        (bind (_bvalid _devicename _applicationinstanceid _devicevisualtype _handindex _trackingstatus _gripposition _griprotation _aimposition _aimrotation) (break `XRMotionControllerData` _motioncontrollerdata))
        (`SceneComponent.K2_SetWorldLocationAndRotation` (`self.WidgetInteractionLeft`) _aimposition (`KismetMathLibrary.Quat_Rotator` _aimrotation) false false)))
    (:`then_1`
      (if (`KismetSystemLibrary.IsValid` _motioncontrollerright)
        (bind _motioncontrollerdata_2 (`HeadMountedDisplayFunctionLibrary.GetMotionControllerData` _motioncontrollerright "Right"))
        (bind (_bvalid_2 _devicename_2 _applicationinstanceid_2 _devicevisualtype_2 _handindex_2 _trackingstatus_2 _gripposition_2 _griprotation_2 _aimposition_2 _aimrotation_2) (break `XRMotionControllerData` _motioncontrollerdata_2))
        (`SceneComponent.K2_SetWorldLocationAndRotation` (`self.WidgetInteractionRight`) _aimposition_2 (`KismetMathLibrary.Quat_Rotator` _aimrotation_2) false false)))))

(event `Key|LeftMouseButton`
  (params (Key :type "Key Structure"))
  (bind _mouseinteraction (`self.MouseInteraction`))
  ;[1 1 1] Interact Mouse input mapping
  (:`Pressed`
    (if (`WidgetInteractionComponent.IsOverInteractableWidget` _mouseinteraction)
      (`WidgetInteractionComponent.PressPointerKey` _mouseinteraction "LeftMouseButton")))
  (:`Released`
    (`WidgetInteractionComponent.ReleasePointerKey` _mouseinteraction "LeftMouseButton")))

(event `InputAction|TriggerLeft`
  (params (Key :type "Key Structure"))
  (bind _widgetinteractionleft (`self.WidgetInteractionLeft`))
  ;[1 1 1] Interact Pointer input mapping
  (:`Pressed`
    (`WidgetInteractionComponent.PressPointerKey` _widgetinteractionleft "LeftMouseButton"))
  (:`Released`
    (`WidgetInteractionComponent.ReleasePointerKey` _widgetinteractionleft "LeftMouseButton")))

(event `InputAction|TriggerRight`
  (params (Key :type "Key Structure"))
  (bind _widgetinteractionright (`self.WidgetInteractionRight`))
  ;[1 1 1] Interact Pointer input mapping
  (:`Pressed`
    (`WidgetInteractionComponent.PressPointerKey` _widgetinteractionright "LeftMouseButton"))
  (:`Released`
    (`WidgetInteractionComponent.ReleasePointerKey` _widgetinteractionright "LeftMouseButton")))

(fn `UserConstructionScript`)