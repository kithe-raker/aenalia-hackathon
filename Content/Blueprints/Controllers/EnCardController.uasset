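; Player controller that spawns and possesses a VR or third-person character at the PlayerStart, based on the game instance's VR flag.
; Non-VR mode also creates the main UI widget, and a cursor toggle switches input mode and shows or resets its panels.
; Pose inputs play emote montages on the BeginPlay third-person character.
; Spectator toggle replaces the current pawn with a newly spawned spectator or third-person pawn in place.
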(event `self.ReceiveBeginPlay`
  ;[1 1 1] init Pawn
  (bind _asaenalia_instance (cast `/Game/Blueprints/AenaliaInstance` (`GameplayStatics.GetGameInstance`)))
  (bind _returnvalue (`GameplayStatics.GetActorOfClass` "/Script/Engine.PlayerStart"))
  (if (`/Game/Blueprints/AenaliaInstance.IsVRMode` _asaenalia_instance)
    (bind _returnvalue_2 (`|SpawnActorFromClass` "/Game/Blueprints/Characters/VRCharacter.VRCharacter_C" (`self.GetTransform` _returnvalue) "Undefined" "OverrideRootScale" null null))
    (`self.Possess` _returnvalue_2)
    (else
      (bind _returnvalue_3 (`|SpawnActorFromClass` "/Game/Blueprints/Characters/ThirdPersonCharacter.ThirdPersonCharacter_C" (`self.GetTransform` _returnvalue) "Undefined" "OverrideRootScale" null null))
      (`self.Possess` _returnvalue_3)
      (bind _returnvalue_4 (`|CreateWidget` "/Game/KyonTest/TestWidget.TestWidget_C"))
      (bind _output_get (set `self.MainUI` _returnvalue_4))
      (`UserWidget.AddToViewport` _output_get 0))))

(event `InputAction|Pose1`
  (params (Key :type "Key Structure"))
  (:`Pressed`
    (`|PlayMontage` (`Character.Mesh` (stale `self.ReceiveBeginPlay` _returnvalue_3)) "/Game/KyonTest/TestPose/Waving/WavingResize_Anim_Montage.WavingResize_Anim_Montage")))

(event `InputAction|Pose4`
  (params (Key :type "Key Structure"))
  (:`Pressed`
    (`|PlayMontage` (`Character.Mesh` (stale `self.ReceiveBeginPlay` _returnvalue_3)) "/Game/KyonTest/TestPose/Dancing/Dancing_Running_Man_Anim_Montage.Dancing_Running_Man_Anim_Montage")))

(event `InputAction|Pose5`
  (params (Key :type "Key Structure"))
  (:`Pressed`
    (`|PlayMontage` (`Character.Mesh` (stale `self.ReceiveBeginPlay` _returnvalue_3)) "/Game/KyonTest/TestPose/Dancing/Samba_Dancing_Anim_Montage.Samba_Dancing_Anim_Montage")))

(event `InputAction|ToggleSpectorMode`
  (params (Key :type "Key Structure"))
  (bind _returnvalue (`self.GetTransform` (`GameplayStatics.GetPlayerPawn` 0)))
  ;[1 1 1] Toggle Spector mode
  (:`Pressed`
    (if (`self.IsEnableSpectorMode`)
      (bind _returnvalue_2 (`|SpawnActorFromClass` "/Game/Blueprints/Characters/ThirdPersonCharacter.ThirdPersonCharacter_C" _returnvalue "AdjustIfPossibleButAlwaysSpawn" "OverrideRootScale" null null))
      (`self.K2_DestroyActor` (`GameplayStatics.GetPlayerPawn` 0))
      (`self.Possess` _returnvalue_2)
      (else
        (bind _returnvalue_3 (`|SpawnActorFromClass` "/Script/Engine.SpectatorPawn" (`KismetMathLibrary.MakeTransform` (.location _returnvalue) (.rotation _returnvalue)) "AdjustIfPossibleButAlwaysSpawn" "OverrideRootScale" null null))
        (`self.K2_DestroyActor` (`GameplayStatics.GetPlayerPawn` 0))
        (`self.Possess` _returnvalue_3)))
    (set `self.IsEnableSpectorMode` (not (`self.IsEnableSpectorMode`)))))

(event `InputAction|Pose3`
  (params (Key :type "Key Structure"))
  (:`Pressed`
    (`|PlayMontage` (`Character.Mesh` (stale `self.ReceiveBeginPlay` _returnvalue_3)) "/Game/KyonTest/TestPose/Backflip/Backflip_Anim_Montage.Backflip_Anim_Montage")))

(event `InputAction|Pose2`
  (params (Key :type "Key Structure"))
  (:`Pressed`
    (`|PlayMontage` (`Character.Mesh` (stale `self.ReceiveBeginPlay` _returnvalue_3)) "/Game/KyonTest/TestPose/Clapping/Clapping_Montage.Clapping_Montage")))

(event `InputAction|ShowMouseCursor`
  (params (Key :type "Key Structure"))
  (:`Pressed`
    (`self.OnShowCursor`)))

(event `OnShowCursor`
  (bind _mainui (`self.MainUI`))
  (bind _bg_button (`/Game/KyonTest/TestWidget.BG_Button` (`self.MainUI`)))
  (`/Engine/EditorBlueprintResources/StandardMacros.FlipFlop`
    (:`A`
      (set `self.bShowMouseCursor` true)
      (`WidgetBlueprintLibrary.SetInputMode_GameAndUIEx` self (`self.MainUI`))
      (`Widget.SetVisibility` _bg_button "Visible"))
    (:`B`
      (set `self.bShowMouseCursor` false)
      (`WidgetBlueprintLibrary.SetInputMode_GameOnly` self)
      (`Widget.SetVisibility` _bg_button "Hidden")
      (`Widget.SetVisibility` (`/Game/KyonTest/TestWidget.CanvasPanelENCardDetail` _mainui) "Hidden")
      (`Widget.SetRenderOpacity` (`/Game/KyonTest/TestWidget.VRModeButton` _mainui) 1.0)
      (`Widget.SetRenderOpacity` (`/Game/KyonTest/TestWidget.RandomENCardButton` _mainui) 1.0)
      (`Widget.SetRenderOpacity` (`/Game/KyonTest/TestWidget.AvatarActionButton` _mainui) 1.0)
      (`Widget.SetVisibility` (`/Game/KyonTest/TestWidget.CanvasPanelAvatarActionDetail` _mainui) "Hidden")
      (`Widget.SetRenderOpacity` (`/Game/KyonTest/TestWidget.ENCardDetailButton` _mainui) 1.0))))

(fn `UserConstructionScript`)